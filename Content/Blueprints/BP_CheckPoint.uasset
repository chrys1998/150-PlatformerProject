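; Checkpoint actor that updates the player's respawn location when BP_Player overlaps it.
; On first overlap it writes its own location, raised on Z, to SpawnPoint in BP_GameInstance and plays a sound there.
; An AlreadyActivated flag makes each checkpoint trigger only once.
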(event `self.ReceiveActorBeginOverlap`
  (params (OtherActor :type "Actor Object Reference"))
  (bind (_returnvalue_x _returnvalue_y _returnvalue_z) (`KismetMathLibrary.BreakVector` (`self.K2_GetActorLocation`)))
  ;[0 0.15 0.1237 0.5] Sets new spawn point when player collides with checkpoint
  (cast `/Game/Blueprints/BP_Player` OtherActor)
  (if (not (`self.AlreadyActivated`))
    (bind _asbp_game_instance (cast `/Game/Blueprints/BP_GameInstance` (`GameplayStatics.GetGameInstance`)))
    (set `/Game/Blueprints/BP_GameInstance.SpawnPoint` (`KismetMathLibrary.MakeVector` _returnvalue_x _returnvalue_y (+ 100.0 _returnvalue_z)) _asbp_game_instance)
    (`GameplayStatics.PlaySoundAtLocation` "/Game/Audio/SFX/surprised-male-wow-reaction-352683.surprised-male-wow-reaction-352683" (`self.K2_GetActorLocation`) (struct) 0.7 1.0 0.0 null null null null)
    (set `self.AlreadyActivated` true)))

(fn `UserConstructionScript`)