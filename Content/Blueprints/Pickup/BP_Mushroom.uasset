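; Mushroom pickup that turns the player into Big Mario.
; Any actor overlap, with no check on the other actor, sets BigMario on player 0's BP_PlayerController, destroys the mushroom and prints a debug string.
; Sphere hits retune ProjectileMovement bounciness by surface normal: low on floor-like surfaces, full on walls and other surfaces, so it rebounds off obstacles.
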(event `self.ReceiveActorBeginOverlap`
  (params (OtherActor :type "Actor Object Reference"))
  (bind _asbp_player_controller (cast `/Game/Blueprints/BP_PlayerController` (`GameplayStatics.GetPlayerController` 0)))
  (set `/Game/Blueprints/BP_PlayerController.BigMario` true _asbp_player_controller)
  (`self.K2_DestroyActor`)
  (`KismetSystemLibrary.PrintString` "Hello"))

(event `self.Sphere1.OnComponentHit`
  (params (HitComponent :type "PrimitiveComponent Object Reference") (OtherActor :type "Actor Object Reference") (OtherComp :type "PrimitiveComponent Object Reference") (NormalImpulse :type "Vector Structure") (Hit :type "HitResult Structure (by ref)"))
  (bind _projectilemovement (`self.ProjectileMovement`))
  (if (> (.z (`.Normal` (`GameplayStatics.BreakHitResult` Hit))) 0.5)
    (set `ProjectileMovementComponent.Bounciness` 0.1 _projectilemovement)
    (else
      (set `ProjectileMovementComponent.Bounciness` 1.0 _projectilemovement))))

(fn `UserConstructionScript`)