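; BP_ScaryCube is an enemy cube that stays idle until something overlaps its CubeSight component, then moves continuously.
; BeginPlay stores the start location, derives EndLocation by subtracting it from a unit Z vector, and disables Tick.
; The overlap enables Tick, which feeds a VInterpTo from the fixed start toward EndLocation at DownSpeed into a swept world offset.
; That interpolated position is applied as a per-frame delta, not an absolute location.
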(event `self.ReceiveBeginPlay`
  (set `self.StartLocation` (`self.K2_GetActorLocation`))
  (set `self.EndLocation` (- (0.0 0.0 1.0) (`self.StartLocation`)))
  (`self.SetActorTickEnabled` false))

(event `self.CubeSight.OnComponentBeginOverlap`
  (params (OverlappedComponent :type "PrimitiveComponent Object Reference") (OtherActor :type "Actor Object Reference") (OtherComp :type "PrimitiveComponent Object Reference") (OtherBodyIndex :type Integer) (bFromSweep :type Boolean) (SweepResult :type "HitResult Structure (by ref)"))
  (`self.SetActorTickEnabled` true))

(event `self.ReceiveTick`
  (params (DeltaSeconds :type "Float (single-precision)"))
  (`self.K2_AddActorWorldOffset` (`KismetMathLibrary.VInterpTo` (`self.StartLocation`) (`self.EndLocation`) DeltaSeconds (`self.DownSpeed`)) true))

(fn `UserConstructionScript`)