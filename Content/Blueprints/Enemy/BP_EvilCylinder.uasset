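; BP_EvilCylinder is an enemy actor set up to move between two points with an InterpToMovement component.
; The construction script adds StartPos and EndPos as relative control points on that component.
; Unconnected event graph nodes would set them to the actor location and a point slightly below it, but BeginPlay is empty, so that logic never runs.
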(event `self.ReceiveBeginPlay`)

(fn `UserConstructionScript`
  (`InterpToMovementComponent.AddControlPointPosition` (`self.InterpToMovement`) (`self.StartPos`) true)
  (`InterpToMovementComponent.AddControlPointPosition` (`self.InterpToMovement`) (`self.EndPos`) true))