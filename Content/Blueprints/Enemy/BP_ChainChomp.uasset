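; BP_ChainChomp is an enemy that follows the player and triggers death through the game instance on overlap.
; Each tick it applies one-hundredth of the offset to the player as a local transform, unswept and frame-rate dependent.
; Overlaps alternate between playing a chomp sound and clearing its flag after a delay.
; A delayed move counter toggles Behavior2, which never gates movement.
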(event `self.ReceiveActorBeginOverlap`
  (params (OtherActor :type "Actor Object Reference"))
  ;[0.15 0 0.003252 0.5] Kills player
  (bind _asbp_player (cast `/Game/Blueprints/BP_Player` OtherActor))
  (`/Engine/EditorBlueprintResources/StandardMacros.IsValid` _asbp_player
    (:`Is Valid`
      (bind _asbp_game_instance (cast `/Game/Blueprints/BP_GameInstance` (`GameplayStatics.GetGameInstance`)))
      (`/Game/Blueprints/BP_GameInstance.Death` _asbp_game_instance)
      (if (`self.SoundDelay`)
        (`KismetSystemLibrary.Delay` 5.0)
        (set `self.SoundDelay` false)
        (else
          (`GameplayStatics.PlaySoundAtLocation` "/Game/Audio/SFX/chain-chomp-made-with-Voicemod.chain-chomp-made-with-Voicemod" (`self.K2_GetActorLocation`) (struct) 0.33 1.0 0.0 null null null null)
          (set `self.SoundDelay` true))))))

(event `self.ReceiveTick`
  (params (DeltaSeconds :type "Float (single-precision)"))
  ; Follows player
  (`/Engine/EditorBlueprintResources/StandardMacros.IsValid` "/Game/Blueprints/BP_Player.BP_Player"
    (:`Is Valid`
      (`|ExecutionSequence`
        (:`then_0`
          (if (`self.Behavior2`)
            (`KismetSystemLibrary.Delay` 7.0)
            (set `self.Behavior2` false)
            (set `self.TimesMoved` 0.0)))
        (:`then_1`
          (`/Engine/EditorBlueprintResources/StandardMacros.IsValid` (`GameplayStatics.GetPlayerPawn` 0)
            (:`Is Valid`
              (`self.K2_AddActorLocalTransform` (`KismetMathLibrary.Conv_VectorToTransform` (/ (- (`self.K2_GetActorLocation` (`GameplayStatics.GetPlayerPawn` 0)) (`self.K2_GetActorLocation`)) (100.0 100.0 100.0)))))))
        (:`then_2`
          (`KismetSystemLibrary.Delay` 0.33)
          (bind _output_get (set `self.TimesMoved` (+ (`self.TimesMoved`) 30.0)))
          (set `self.Behavior2` (>= _output_get 50.0)))))))

(fn `UserConstructionScript`)