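; Player controller for a Mario-style side-scroller that moves the pawn with swept world offsets for walking, jumping and gravity.
; Horizontal input ramps speed toward a maximum set, like jump height, by sprint and Big Mario state.
; Space runs a Delay-looped jump with a counter and, with FirePower, spawns BP_Mushroom.
; Events grant fire power or timed invincibility; Tick updates scale, limits and jump availability only while falling.
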(event `Key|SpaceBar`
  (params (Key :type "Key Structure"))
  ; Handles all movement related scripts for the character
  ;;[1 0.3277 0 0.5] Will Spawn Fireball from Component
  (:`Pressed`
    (if (`self.FirePower`)
      (bind _asbp_player (cast `/Game/Blueprints/BP_Player` (`GameplayStatics.GetPlayerPawn` 0)))
      (`|SpawnActorFromClass` "/Game/Blueprints/Pickup/BP_Mushroom.BP_Mushroom_C" (`KismetMathLibrary.Conv_VectorToTransform` (`SceneComponent.GetRightVector` (`SceneComponent.GetChildComponent` (`/Game/Blueprints/BP_Player.Cube1` _asbp_player) 0))) "Undefined" "MultiplyWithRoot" null null))))

(event `Key|A`
  (params (Key :type "Key Structure"))
  ; Handles all movement related scripts for the character
  ;;[0 0.1349 0.4635 0.5] Reset movement speed during breaks in movement
  (:`Pressed`
    (if (`self.SprintEnabled`) :!label _label
      (set `self.MoveSpeed` 200.0)
      (else
        (set `self.MoveSpeed` 50.0)))))

(event `Fire`
  ; Handles all movement related scripts for the character
  ;;[1 0.005894 0 0.5] Gives Mario Fire Power
  (set `self.FirePower` true)
  (set `self.BigMario` true))

(event `Key|LeftShift`
  (params (Key :type "Key Structure"))
  ; Handles all movement related scripts for the character
  ;;[0.9111 1 0 0.5] Hold Shift to Sprint
  (:`Pressed`
    (set `self.SprintEnabled` true))
  (:`Released`
    (set `self.SprintEnabled` false)))

(event `Key|D`
  (params (Key :type "Key Structure"))
  ; Handles all movement related scripts for the character
  ;;[0 0.1349 0.4635 0.5] Reset movement speed during breaks in movement
  (:`Pressed`
    (goto _label)))

(event `Invincibility`
  ; Handles all movement related scripts for the character
  ;;[0.9115 0 0.7148 0.5] Sets player to be invincible for 30 seconds
  (set `self.Invincible` true)
  (`KismetSystemLibrary.Delay` 30.0)
  (set `self.Invincible` false))

(event `InputAxis|HorizontalInput`
  (params (AxisValue :type "Float (single-precision)"))
  (bind _movespeed (`self.MoveSpeed`))
  ; Handles all movement related scripts for the character
  ;;[0.004615 0.3646 0 0.5] Sets input value for movement
  (set `self.MoveDirection` (`KismetMathLibrary.MakeVector` 0.0 AxisValue))
  ;;[0.9489 0.9688 0 0.5] If player movement speed is less than maximum movement speed, ramps it up while horizontal input is held
  (`/Engine/EditorBlueprintResources/StandardMacros.CompareFloat` _movespeed (`self.MaxMoveSpeed`)
    (:`<`
      (set `self.MoveSpeed` (+ _movespeed (/ (- (`self.MaxMoveSpeed`) (`self.MoveSpeed`)) 50.0))))))

(event `self.ReceiveTick`
  (params (DeltaSeconds :type "Float (single-precision)"))
  (bind _returnvalue (`GameplayStatics.GetPlayerPawn` 0))
  (bind _returnvalue_2 (`GameplayStatics.GetPlayerPawn` 0))
  (bind _returnvalue_3 (`GameplayStatics.GetPlayerPawn` 0))
  (bind (_movedirection_x _movedirection_y) (`KismetMathLibrary.BreakVector` (`self.MoveDirection`)))
  (bind _jumptimes (`self.JumpTimes`))
  ; Handles all movement related scripts for the character
  ;;[0.000886 0.3281 0.0536 0.5] Controls movement
  (`/Engine/EditorBlueprintResources/StandardMacros.IsValid` _returnvalue_2
    (:`Is Valid`
      (`self.K2_AddActorWorldOffset` _returnvalue_2 (`KismetMathLibrary.MakeVector` 0.0 (* DeltaSeconds _movedirection_y (`self.MoveSpeed`))) true false)
      ;;[0 0.2024 0.3854 0.5] If player is falling, applies gravity
      (if (`self.IsFalling`)
        (`/Engine/EditorBlueprintResources/StandardMacros.IsValid` _returnvalue_3
          (:`Is Valid`
            (`self.K2_AddActorWorldOffset` _returnvalue_3 (`KismetMathLibrary.MakeVector` 0.0 0.0 (* DeltaSeconds (`self.Gravity`))) true false)
            (`/Engine/EditorBlueprintResources/StandardMacros.IsValid` (`GameplayStatics.GetPlayerPawn` 0)
              (:`Is Valid`
                ;;[0 1 0.8569 0.5] Sets size of Mario
                (if (`self.BigMario`)
                  (`self.SetActorScale3D` _returnvalue (0.5 0.67 1.33))
                  (else
                    (`self.SetActorScale3D` _returnvalue (0.5 0.5 1.0))))
                ;;[1 0.9143 0.004255 0.5] Sets Max Movement Speed based on the Sprint bool
                (if (`self.SprintEnabled`)
                  (if (`self.BigMario`)
                    (set `self.MaxMoveSpeed` 900.0)
                    (set `self.JumpHeight` 700.0)
                    (else
                      (set `self.MaxMoveSpeed` 600.0)
                      (set `self.JumpHeight` 450.0)))
                  (elif (`self.BigMario`)
                    (set `self.MaxMoveSpeed` 600.0)
                    (set `self.JumpHeight` 450.0)
                    (else
                      (set `self.MaxMoveSpeed` 400.0)
                      (set `self.JumpHeight` 300.0))))
                ;;[0.375 0 0.1076 0.5] Checks if player can jump
                (`/Engine/EditorBlueprintResources/StandardMacros.CompareInt` _jumptimes 2
                  (:`>`
                    (set `self.CanJump` false :!label _label_2)
                    (`KismetSystemLibrary.Delay` 0.5)
                    (`/Engine/EditorBlueprintResources/StandardMacros.DecrementInt` _jumptimes))
                  (:`==`
                    (goto _label_2))
                  (:`<`
                    (set `self.CanJump` true)))))))))))

(event `Key|SpaceBar`
  (params (Key :type "Key Structure"))
  (bind _returnvalue (`GameplayStatics.GetPlayerPawn` 0))
  (bind _returnvalue_2 (`GameplayStatics.GetPlayerPawn` 0))
  (bind _jumpfraction (`self.JumpFraction`))
  ; Handles all movement related scripts for the character
  ;;[0 0.4167 0.1525 0.5] Character jumps when spacebar is pressed
  (:`Pressed`
    (if (`self.CanJump`)
      ;;;[0 0.002385 0.3542 0.5] Plays SFX after jumping
      (`/Engine/EditorBlueprintResources/StandardMacros.IsValid` _returnvalue
        (:`Is Valid`
          (`GameplayStatics.PlaySoundAtLocation` "/Game/Audio/SFX/maro-jump-sound-effect_1.maro-jump-sound-effect_1" (`self.K2_GetActorLocation` _returnvalue) (struct) 0.5 1.0 0.0 null null null null)
          ;;;[0.3385 0 0.09211 0.5] Handles the jump counter and falling status
          (`/Engine/EditorBlueprintResources/StandardMacros.IncrementInt` (`self.JumpTimes`)
            (:`  `
              (set `self.IsFalling` false)
              ;;;[0.1128 0.15 0 0.5] Outputs fraction of jump height, and adds to total for tracking purposes
              (set `self.JumpTotal` (+ _jumpfraction (`self.JumpTotal`)) :!label _label_3)
              (`/Engine/EditorBlueprintResources/StandardMacros.IsValid` _returnvalue_2
                (:`Is Valid`
                  (`self.K2_AddActorWorldOffset` _returnvalue_2 (`KismetMathLibrary.MakeVector` 0.0 0.0 _jumpfraction) true false)
                  ;;;[0.6979 0 0.04054 0.5] Continues through jump until jump total equals jump height
                  (if (>= (`self.JumpTotal`) (`self.JumpHeight`))
                    ;;;;[0.001352 0.1764 0.4948 0.5] Reset
                    (set `self.IsFalling` true)
                    (set `self.JumpTotal` 0.0)
                    (else
                      (`KismetSystemLibrary.Delay` 0.0001)
                      (goto _label_3))))))))))))

(fn `UserConstructionScript`)