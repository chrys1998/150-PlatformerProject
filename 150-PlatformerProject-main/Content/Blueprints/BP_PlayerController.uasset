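; Player controller that drives a pawn along the Y axis with sprinting, jumping and simple gravity.
; Horizontal input sets direction and eases speed toward a cap, while A/D presses reset starting speed based on Shift sprint.
; Tick moves the pawn by swept world offsets and, while falling, applies gravity, updates the speed cap and limits jumps through a counter decremented after a Delay.
; Space applies an instant upward offset and plays a sound.
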(event `Key|A`
  (params (Key :type "Key Structure"))
  ; Handles all movement related scripts for the character
  ;;[0 0.1349 0.4635 0.5] Reset movement speed during breaks in movement
  (:`Pressed`
    (if (`self.SprintEnabled`) :!label _label
      (set `self.MoveSpeed` 200.0)
      (else
        (set `self.MoveSpeed` 5.0)))))

(event `Key|LeftShift`
  (params (Key :type "Key Structure"))
  ; Handles all movement related scripts for the character
  ;;[0.9111 1 0 0.5] Hold Shift to Sprint
  (:`Pressed`
    (set `self.SprintEnabled` true))
  (:`Released`
    (set `self.SprintEnabled` false)))

(event `Key|D`
  (params (Key :type "Key Structure"))
  ; Handles all movement related scripts for the character
  ;;[0 0.1349 0.4635 0.5] Reset movement speed during breaks in movement
  (:`Pressed`
    (goto _label)))

(event `InputAxis|HorizontalInput`
  (params (AxisValue :type "Float (single-precision)"))
  (bind _movespeed (`self.MoveSpeed`))
  ; Handles all movement related scripts for the character
  ;;[0.004615 0.3646 0 0.5] Sets input value for movement
  (set `self.MoveDirection` (`KismetMathLibrary.MakeVector` 0.0 AxisValue))
  ;;[0.9489 0.9688 0 0.5] If player movement speed is less than maximum movement speed, ramps it up while horizontal input is held
  (`/Engine/EditorBlueprintResources/StandardMacros.CompareFloat` _movespeed (`self.MaxMoveSpeed`)
    (:`<`
      (set `self.MoveSpeed` (+ _movespeed (/ (- (`self.MaxMoveSpeed`) (`self.MoveSpeed`)) 100.0))))))

(event `self.ReceiveTick`
  (params (DeltaSeconds :type "Float (single-precision)"))
  (bind (_movedirection_x _movedirection_y) (`KismetMathLibrary.BreakVector` (`self.MoveDirection`)))
  (bind _jumptimes (`self.JumpTimes`))
  ; Handles all movement related scripts for the character
  ;;[0.000886 0.3281 0.0536 0.5] Controls movement
  (`self.K2_AddActorWorldOffset` (`GameplayStatics.GetPlayerPawn` 0) (`KismetMathLibrary.MakeVector` 0.0 (* DeltaSeconds _movedirection_y (`self.MoveSpeed`))) true false)
  ;;[0 0.2024 0.3854 0.5] If player is falling, applies gravity
  (if (`self.IsFalling`)
    (`self.K2_AddActorWorldOffset` (`GameplayStatics.GetPlayerPawn` 0) (`KismetMathLibrary.MakeVector` 0.0 0.0 (* DeltaSeconds (`self.Gravity`))) true false)
    ;;[1 0.9143 0.004255 0.5] Sets Max Movement Speed based on the Sprint bool
    (if (`self.SprintEnabled`)
      (set `self.MaxMoveSpeed` 800.0)
      (else
        (set `self.MaxMoveSpeed` 400.0)))
    ;;[0.375 0 0.1076 0.5] Checks if player can jump
    (`/Engine/EditorBlueprintResources/StandardMacros.CompareInt` (`self.JumpTimes`) 2
      (:`>`
        (set `self.CanJump` false :!label _label_2))
      (:`==`
        (goto _label_2))
      (:`<`
        (set `self.CanJump` true)))
    (`KismetSystemLibrary.Delay` 1.0)
    (`/Engine/EditorBlueprintResources/StandardMacros.CompareInt` _jumptimes
      (:`>`
        (`/Engine/EditorBlueprintResources/StandardMacros.DecrementInt` _jumptimes)))))

(event `Key|SpaceBar`
  (params (Key :type "Key Structure"))
  ; Handles all movement related scripts for the character
  ;;[0 0.4167 0.1525 0.5] Character jumps when spacebar is pressed
  (:`Pressed`
    (if (`self.CanJump`)
      (set `self.IsFalling` false)
      (`self.K2_AddActorWorldOffset` (`GameplayStatics.GetPlayerPawn` 0) (`KismetMathLibrary.MakeVector` 0.0 0.0 (`self.JumpHeight`)) false false)
      (set `self.IsFalling` true)
      ;;[0 0.002385 0.3542 0.5] Plays SFX after jumping
      (`GameplayStatics.PlaySoundAtLocation` "/Game/Audio/SFX/maro-jump-sound-effect_1.maro-jump-sound-effect_1" (`self.K2_GetActorLocation` (`GameplayStatics.GetPlayerPawn` 0)) (struct) 1.0 1.0 0.0 null null null null)
      ;;[0.3385 0 0.09211 0.5] Handles the jump counter
      (`/Engine/EditorBlueprintResources/StandardMacros.IncrementInt` (`self.JumpTimes`)))))

(fn `UserConstructionScript`)